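; Firearm weapon Blueprint that extends a parent weapon with ammo, spread, recoil and reloading.
; UseWeapon spawns FireProjectile if set, otherwise applies point damage via a camera-origin line trace, both using randomized spread around the owner's forward vector.
; An empty magazine sets Reloading, whose OnRep starts an authority-only timer that refills toward the class-default CurrentAmmo from TotalAmmo.
; OwnerWeaponUsed plays a timeline that adds recoil pitch to the weapon owner.
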(event Custom|DEBUS_DrawServerTrace
  (params (Start :type Vector) (End :type Vector) (Hit :type Vector))
  (Rendering|Debug|DrawDebugLine Start End "(R=0.954200,G=1.000000,B=0.168114,A=1.000000)" 5.0 2.0)
  (Rendering|Debug|DrawDebugSphere Hit 4e+01 8 "(R=1.000000,G=0.021743,B=0.000000,A=1.000000)" 5.0 2.0))

(event EventOwnerWeaponUsed
  (|CallParentFunction)
  (if (CallFunction|AbletoUseWeapon)
    (bind _lerp (Timeline|Timeline PlayFromStart)
      (:Update
        (Pawn|Input|AddControllerPitchInput (Variables|Default|GetWeaponOwner) (* _lerp (Variables|Default|GetRecoil) -1.0))))))

(fn ConstructionScript
  (|CallParentFunction))

(fn UseWeapon
  (bind _used (|CallParentFunction))
  (CallFunction|PrintMessage (Utilities|String|Append (Utilities|String|ToString(Integer) (Variables|Default|GetCurrentAmmo)) "|" (Utilities|String|ToString(Integer) (Variables|Default|GetTotalAmmo))) "(R=0.040298,G=0.088876,B=0.264730,A=1.000000)" 1.0 false)
  (if _used
    (if (Utilities|IsValidClass (Variables|Default|GetFireProjectile))
      (CallFunction|SpawnShootProjectile)
      (return true)
      (else
        (CallFunction|ShootFireTrace)
        (return true)))
    (elif (and (<= (Variables|Default|GetCurrentAmmo) 0) (> (Variables|Default|GetTotalAmmo) 0))
      (Variables|Reload|SetReloading true)
      (return false)
      (else
        (return false)))))

(fn ShootFireTrace
  (bind _asbp_player_character (Utilities|Casting|CastToBP_PlayerCharacter (Game|GetInstigator))
    (:then
      (bind _outhit (Collision|LineTraceForObjects (Transformation|GetWorldLocation (Variables|/Game/Blueprints/Player/BP_PlayerCharacter.BP_PlayerCharacter_C|GetCamera _asbp_player_character)) (+ (Transformation|GetWorldLocation (Variables|/Game/Blueprints/Player/BP_PlayerCharacter.BP_PlayerCharacter_C|GetCamera _asbp_player_character)) (* (CallFunction|GetShootDirection) 1e+04)) (Utilities|Array|MakeArray "ObjectTypeQuery1" "ObjectTypeQuery2" "ObjectTypeQuery3") false (Utilities|Array|MakeArray self (Game|GetInstigator)) "None"))
      (Game|Damage|ApplyPointDamage (.HitActor (Collision|BreakHitResult _outhit)) (Variables|Default|GetDamage) (Math|Vector|GetUnitDirection(Vector) (.TraceEnd (Collision|BreakHitResult _outhit)) (.TraceStart (Collision|BreakHitResult _outhit))) _outhit (Game|GetInstigatorController) self)
      (return))
    (:CastFailed
      (return))))

(fn Reload
  (Variables|Reload|SetReloading true))

(fn ReloadFinished
  (Variables|Reload|SetReloading false)
  (Variables|Default|SetCurrentAmmo (+ (Variables|Default|GetCurrentAmmo) (Variables|Reload|GetAmmoToReload)))
  (Variables|Default|SetTotalAmmo (- (Variables|Default|GetTotalAmmo) (Variables|Reload|GetAmmoToReload))))

(fn OnRepReloading
  (Networking|SwitchHasAuthority
    (:Authority
      (if (Variables|Reload|GetReloading)
        (if (CallFunction|AbletoReload)
          (CallFunction|PrintMessage "Reloading" "(R=0.064988,G=0.608162,B=0.629537,A=1.000000)" 2.0 false)
          (bind _returnvalue (Utilities|Time|SetTimerbyFunctionName 0 "ReloadFinished" (Variables|Reload|GetReloadTime)))
          (Variables|Reload|SetReloadTimer _returnvalue)
          (Variables|Reload|SetAmmoToReload (Math|Integer|Min(Integer) (- (.CurrentAmmo (Utilities|GetClassDefaults (Utilities|GetClass self))) (Variables|Default|GetCurrentAmmo)) (Variables|Default|GetTotalAmmo)))
          (else
            (Variables|Reload|SetReloading false)
            (CallFunction|PrintMessage "Not able to reload" "(R=0.064988,G=0.608162,B=0.629537,A=1.000000)" 2.0 true)))
        (else
          (Utilities|Time|ClearandInvalidateTimerbyHandle (Variables|Reload|GetReloadTimer)))))))

(fn AbletoReload
  (return (Math|Boolean|ANDBoolean (!= (.CurrentAmmo (Utilities|GetClassDefaults (Utilities|GetClass self))) (Variables|Default|GetCurrentAmmo)) (> (Variables|Default|GetTotalAmmo) 0) (not (Utilities|Time|IsValidTimerHandle (Variables|Reload|GetReloadTimer))))))

(fn AbletoUseWeapon
  (return (and (|CallParentFunction) (not (Variables|Reload|GetReloading)))))

(fn SpawnShootProjectile
  (bind _asbp_player_character (Utilities|Casting|CastToBP_PlayerCharacter (Game|GetInstigator)))
  (Game|SpawnActorfromClass (Variables|Default|GetFireProjectile) (Math|Transform|MakeTransform (+ (Transformation|GetWorldLocation (Variables|/Game/Blueprints/Player/BP_PlayerCharacter.BP_PlayerCharacter_C|GetCamera _asbp_player_character)) (* (Transformation|GetActorForwardVector (Components|GetOwner)) 7e+01)) (Math|Conversions|RotationFromXVector (CallFunction|GetShootDirection))) "AlwaysSpawn" self (Variables|Default|GetDamage) (Game|GetInstigator)))

(fn GetShootDirection
  (bind _returnvalue (Components|GetOwner))
  (bind _spreadangle (Variables|Default|GetSpreadAngle))
  (bind _spreadangle_2 (Variables|Default|GetSpreadAngle))
  (return (Math|Vector|RotateVectorAroundAxis (Math|Vector|RotateVectorAroundAxis (Transformation|GetActorForwardVector _returnvalue) (Math|Random|RandomFloatinRange (* _spreadangle_2 -1.0) _spreadangle_2) (Transformation|GetActorRightVector _returnvalue)) (Math|Random|RandomFloatinRange (* _spreadangle -1.0) _spreadangle) (Transformation|GetActorUpVector _returnvalue))))