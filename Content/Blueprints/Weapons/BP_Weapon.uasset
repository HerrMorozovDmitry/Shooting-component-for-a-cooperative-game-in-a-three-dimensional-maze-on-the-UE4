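; BP_Weapon is a weapon Blueprint that handles ammo consumption and use-rate limiting, with no firing effects of its own.
; UseWeapon checks AbleToUseWeapon, spends one round of CurrentAmmo, locks further use and returns whether it succeeded.
; A timer set by function name calls StopRateDelay after UseRate to clear the lock.
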(event EventBeginPlay)

(event Collision|EventActorBeginOverlap
  (params (OtherActor :type Actor%20Object%20Reference)))

(event EventTick
  (params (DeltaSeconds :type Float%20%28single-precision%29)))

(fn ConstructionScript)

(fn UseWeapon
  (if (CallFunction|AbletoUseWeapon)
    (Math|Integer|DecrementInt (Variables|Default|GetCurrentAmmo)
      (:%20%20
        (Utilities|Time|SetTimerbyFunctionName 0 "StopRateDelay" (Variables|Default|GetUseRate))
        (Variables|Default|SetUsedFreezedByRate true)
        (return true)))
    (else
      (return false))))

(fn AbletoUseWeapon
  (return (and (> (Variables|Default|GetCurrentAmmo) 0) (not (Variables|Default|GetUsedFreezedByRate)))))

(fn StopRateDelay
  (Variables|Default|SetUsedFreezedByRate false))